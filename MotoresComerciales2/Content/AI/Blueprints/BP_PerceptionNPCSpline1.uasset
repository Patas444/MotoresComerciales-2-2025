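; BP_PerceptionNPCSpline1 is an NPC actor that places its Character component on a Spline component.
; Each Tick samples the spline's local transform and applies it to the Character, with height and yaw offsets and its scale preserved.
; DistanceAlongSpline is reset to zero every frame and the speed-based increment is left unconnected, so the Character stays at the spline's start.
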(event EventTick
  (params (DeltaSeconds :type Float%20%28single-precision%29))
  (Variables|Components|SetDistanceAlongSpline 0.0)
  (Transformation|SetRelativeTransform (Variables|Default|GetCharacter) (Math|Transform|MakeTransform (Math|Vector|MakeVector (.x (.location (Spline|GetTransformatDistanceAlongSpline (Variables|Default|GetSpline) (Variables|Components|GetDistanceAlongSpline) "Local" false))) (.y (.location (Spline|GetTransformatDistanceAlongSpline (Variables|Default|GetSpline) (Variables|Components|GetDistanceAlongSpline) "Local" false))) (+ (.z (.location (Spline|GetTransformatDistanceAlongSpline (Variables|Default|GetSpline) (Variables|Components|GetDistanceAlongSpline) "Local" false))) -89.0)) (Math|Rotator|MakeRotator (.roll (.rotation (Spline|GetTransformatDistanceAlongSpline (Variables|Default|GetSpline) (Variables|Components|GetDistanceAlongSpline) "Local" false))) (.pitch (.rotation (Spline|GetTransformatDistanceAlongSpline (Variables|Default|GetSpline) (Variables|Components|GetDistanceAlongSpline) "Local" false))) (+ (.yaw (.rotation (Spline|GetTransformatDistanceAlongSpline (Variables|Default|GetSpline) (Variables|Components|GetDistanceAlongSpline) "Local" false))) -9e+01)) (Variables|/Script/Engine.SceneComponent|GetRelativeScale3D (Variables|Default|GetCharacter))) false false))

(event Collision|EventActorBeginOverlap
  (params (OtherActor :type Actor%20Object%20Reference)))

(event EventBeginPlay)

(fn ConstructionScript)