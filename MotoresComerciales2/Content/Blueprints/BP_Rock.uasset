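; BP_Rock is a rock actor that simulates gradual snow accumulation on its surface after play begins.
; The construction script creates a dynamic instance of M_Moss_Inst on the Cube mesh and stores it as SnowMaterial.
; A looping half-second timer calls SnowAcumulation, which nudges the material's "Blend Sharpness (S)" parameter upward.
; BeginPlay clears that timer after a 30-second delay, ending the buildup.
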(event EventBeginPlay
  (bind _returnvalue (Utilities|Time|SetTimerbyFunctionName 0 "SnowAcumulation" 0.5 true))
  (Utilities|FlowControl|Delay 3e+01)
  (Utilities|Time|ClearandInvalidateTimerbyHandle _returnvalue))

(event Collision|EventActorBeginOverlap
  (params (OtherActor :type Actor%20Object%20Reference)))

(event EventTick
  (params (DeltaSeconds :type Float%20%28single-precision%29)))

(fn ConstructionScript
  (bind _returnvalue (Rendering|Material|CreateDynamicMaterialInstance (Variables|Default|GetCube) 0 "/Game/Materiales/Blend/M_Moss_Inst.M_Moss_Inst" "None" :!class /Script/Engine.PrimitiveComponent))
  (Variables|Default|SetSnowMaterial _returnvalue))

(fn SnowAcumulation
  (bind _snowmaterial (Variables|Default|GetSnowMaterial))
  (bind _returnvalue (Rendering|Material|GetScalarParameterValue _snowmaterial "Blend Sharpness (S)" :!class /Script/Engine.MaterialInstanceDynamic))
  (Rendering|Material|SetScalarParameterValue _snowmaterial "Blend Sharpness (S)" (+ _returnvalue 0.01) :!class /Script/Engine.MaterialInstanceDynamic))